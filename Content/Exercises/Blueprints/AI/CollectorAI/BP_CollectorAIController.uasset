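; AI controller for the collector AI that fetches items on the player's request.
; On possess it runs the BT_CollectorAI behavior tree.
; On BeginPlay it binds to the player's OnPickupRequest event dispatcher, then writes the requested item and a has-order flag to the blackboard for the tree to act on.
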(event `self.ReceivePossess`
  (params (PossessedPawn :type "Pawn Object Reference"))
  (`self.RunBehaviorTree` "/Game/Exercises/Blueprints/AI/CollectorAI/BT_CollectorAI.BT_CollectorAI"))

(event `self.ReceiveBeginPlay`
  (bind _asbp_player (cast `/Game/Exercises/Blueprints/BP_Player` (`GameplayStatics.GetPlayerCharacter` 0)))
  (add `/Game/Exercises/Blueprints/BP_Player.OnPickupRequest` _asbp_player (delegate `OnPickupRequest_Event`)))

(event `OnPickupRequest_Event`
  (params (TargetItem :type "Actor Object Reference"))
  (`BlackboardComponent.SetValueAsBool` (`self.Blackboard`) (`self.HasOrderKey`) true)
  (`BlackboardComponent.SetValueAsObject` (`self.Blackboard`) (`self.TargetItemKey`) TargetItem))

(fn `UserConstructionScript`)