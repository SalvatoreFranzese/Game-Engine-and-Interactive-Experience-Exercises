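; Collector AI character that keeps an item inventory and shows it on screen while the player is nearby.
; Player overlap with its Sphere creates WBP_Inventory bound to this AI and enables the cursor with Game and UI input; leaving reverses this.
; Helper functions set walk speed, add or remove inventory items, and drop the equipped item by spawning a same-class copy at an offset and destroying the original.
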(event `self.Sphere.OnComponentBeginOverlap`
  (params (OverlappedComponent :type "PrimitiveComponent Object Reference") (OtherActor :type "Actor Object Reference") (OtherComp :type "PrimitiveComponent Object Reference") (OtherBodyIndex :type Integer) (bFromSweep :type Boolean) (SweepResult :type "HitResult Structure (by ref)"))
  ; Inventory UI
  (cast `/Game/Exercises/Blueprints/BP_Player` OtherActor)
  (bind _returnvalue (`|CreateWidget` "/Game/Exercises/Blueprints/AI/CollectorAI/UI/WBP_Inventory.WBP_Inventory_C" null self))
  (bind _output_get (set `self.InventoryUI` _returnvalue))
  (`UserWidget.AddToViewport` _output_get 0)
  (set `PlayerController.bShowMouseCursor` true (`GameplayStatics.GetPlayerController` 0))
  (`WidgetBlueprintLibrary.SetInputMode_GameAndUIEx` (`GameplayStatics.GetPlayerController` 0) null))

(event `self.Sphere.OnComponentEndOverlap`
  (params (OverlappedComponent :type "PrimitiveComponent Object Reference") (OtherActor :type "Actor Object Reference") (OtherComp :type "PrimitiveComponent Object Reference") (OtherBodyIndex :type Integer))
  ; Inventory UI
  (cast `/Game/Exercises/Blueprints/BP_Player` OtherActor)
  (`Widget.RemoveFromParent` (`self.InventoryUI`))
  (set `PlayerController.bShowMouseCursor` false (`GameplayStatics.GetPlayerController` 0))
  (`WidgetBlueprintLibrary.SetInputMode_GameOnly` (`GameplayStatics.GetPlayerController` 0) true))

(fn `AddToInventory`
  (params (Item :type "/Game/Exercises/Blueprints/AI/CollectorAI/Collectibles/BP_CollectibleBase Object Reference"))
  (`KismetArrayLibrary.Array_Add` (`self.Inventory`) Item))

(fn `DropEquippedItem`
  (bind (_returnvalue_x _returnvalue_y) (`KismetMathLibrary.BreakVector` (+ (`self.K2_GetActorLocation`) (50.0 0.0 0.0))))
  (`|SpawnActorFromClass` (`GameplayStatics.GetObjectClass` (`self.EquippedItem`)) (`KismetMathLibrary.MakeTransform` (`KismetMathLibrary.MakeVector` _returnvalue_x _returnvalue_y)) "Undefined" "MultiplyWithRoot" null null)
  (`self.K2_DestroyActor` (`self.EquippedItem`)))

(fn `RemoveFromInventory`
  (params (Index :type Integer))
  (`KismetArrayLibrary.Array_Remove` (`self.Inventory`) Index))

(fn `UpdateWalkSpeed`
  (params (Speed :type "Float (double-precision)"))
  (set `CharacterMovementComponent.MaxWalkSpeed` Speed (`self.CharacterMovement`)))

(fn `UserConstructionScript`)