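; AI controller for an enemy that runs the BT_Enemy behavior tree on possess and feeds it player sighting data.
; AI perception updates set the HasLineOfSight and PlayerActor blackboard keys when a Player-tagged actor is sensed, cancelling any pending lose-sight timer.
; Any other perception update starts that timer, which clears both keys on expiry to give a grace period before the enemy forgets the player.
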(event `self.ReceivePossess`
  (params (PossessedPawn :type "Pawn Object Reference"))
  (`self.RunBehaviorTree` "/Game/Exercises/Blueprints/AI/Enemy/BT_Enemy.BT_Enemy"))

(event `self.AIPerception.OnTargetPerceptionUpdated`
  (params (Actor :type "Actor Object Reference") (Stimulus :type "AIStimulus Structure"))
  (if (and (`self.ActorHasTag` Actor "Player") (`.bSuccessfullySensed` (break `AIStimulus` Stimulus)))
    (`KismetSystemLibrary.K2_ClearAndInvalidateTimerHandle` (`self.EnemyTimer`))
    (`BlackboardComponent.SetValueAsBool` (`self.Blackboard`) (`self.HasLineOfSight`) true)
    (`BlackboardComponent.SetValueAsObject` (`self.Blackboard`) (`self.PlayerActor`) Actor)
    (else
      (bind _returnvalue (`KismetSystemLibrary.K2_SetTimerDelegate` (delegate `StartLoseSightTimer`) (`self.LineOfSightTimer`)))
      (set `self.EnemyTimer` _returnvalue))))

(event `StartLoseSightTimer`
  (`BlackboardComponent.SetValueAsBool` (`self.Blackboard`) (`self.HasLineOfSight`) false)
  (`BlackboardComponent.SetValueAsObject` (`self.Blackboard`) (`self.PlayerActor`) null))

(fn `UserConstructionScript`)