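; AI controller for a pickup agent that fetches items on the player's request.
; On possess it runs the BT_AIPickup behavior tree.
; At BeginPlay it binds to the player character's OnPickupRequest dispatcher.
; Each request sets a HasOrder flag and stores the target item in the blackboard for the tree to act on.
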(event `self.ReceivePossess`
  (params (PossessedPawn :type "Pawn Object Reference"))
  (`self.RunBehaviorTree` "/Game/Exercises/Blueprints/AI/AIPickup/BT_AIPickup.BT_AIPickup"))

(event `self.ReceiveBeginPlay`
  (bind _asbp_third_person_character_child (cast `/Game/Exercises/Blueprints/BP_ThirdPersonCharacter_Child` (`GameplayStatics.GetPlayerCharacter` 0)))
  (add `/Game/Exercises/Blueprints/BP_ThirdPersonCharacter_Child.OnPickupRequest` _asbp_third_person_character_child (delegate `OnPickupRequest_Event`)))

(event `OnPickupRequest_Event`
  (params (TargetItem :type "Actor Object Reference"))
  (`BlackboardComponent.SetValueAsBool` (`self.Blackboard`) (`self.HasOrderKey`) true)
  (`BlackboardComponent.SetValueAsObject` (`self.Blackboard`) (`self.TargetItemKey`) TargetItem))

(fn `UserConstructionScript`)