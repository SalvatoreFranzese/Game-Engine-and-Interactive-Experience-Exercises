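; AI controller for a companion character that follows the player.
; On possess it runs the BT_Companion behavior tree, and AI perception updates write to its Blackboard.
; A sensed Player-tagged actor becomes the target, while any other update falls back to player pawn 0.
; Both branches set the follow key true, so perception never switches following off.
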(event `self.ReceivePossess`
  (params (PossessedPawn :type "Pawn Object Reference"))
  (`self.RunBehaviorTree` "/Game/Exercises/Blueprints/AI/Companion/BT_Companion.BT_Companion"))

(event `self.AIPerception.OnTargetPerceptionUpdated`
  (params (Actor :type "Actor Object Reference") (Stimulus :type "AIStimulus Structure"))
  (if (and (`self.ActorHasTag` Actor "Player") (`.bSuccessfullySensed` (break `AIStimulus` Stimulus)))
    (`BlackboardComponent.SetValueAsBool` (`self.Blackboard`) (`self.FollowKey`) true)
    (`BlackboardComponent.SetValueAsObject` (`self.Blackboard`) (`self.TargetKey`) Actor)
    (else
      (`BlackboardComponent.SetValueAsBool` (`self.Blackboard`) (`self.FollowKey`) true)
      (`BlackboardComponent.SetValueAsObject` (`self.Blackboard`) (`self.TargetKey`) (`GameplayStatics.GetPlayerPawn` 0)))))

(fn `UserConstructionScript`)