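; Player character Blueprint with overlap-based interaction, line-trace pickup requests, an over-the-shoulder aim camera and an enemy motion tracker.
; The motion tracker stores an overlapping enemy and drives an audio "Distance" parameter from inverted, normalized proximity on Tick.
; A GM_EX callback sets target progress from points, which Tick interpolates into the GameStateBar's dynamic material for a smooth fill.
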(event OnComponentBeginOverlap(CapsuleComponent)
  (params (OverlappedComponent :type Primitive%20Component%20Object%20Reference) (OtherActor :type Actor%20Object%20Reference) (OtherComp :type Primitive%20Component%20Object%20Reference) (OtherBodyIndex :type Integer) (bFromSweep :type Boolean) (SweepResult :type Hit%20Result%20Structure%20%28by%20ref%29))
  ;[0.15 0.15 0.15 0.5] Interact
  (bind _asbp_interactable_base (Utilities|Casting|CastToBP_InteractableBase OtherActor))
  (Variables|Default|SetBP_Interactable%20Base _asbp_interactable_base)
  (Variables|Default|SetIsInteracting true))

(event OnComponentEndOverlap(CapsuleComponent)
  (params (OverlappedComponent :type Primitive%20Component%20Object%20Reference) (OtherActor :type Actor%20Object%20Reference) (OtherComp :type Primitive%20Component%20Object%20Reference) (OtherBodyIndex :type Integer))
  ;[0.15 0.15 0.15 0.5] Interact
  (Variables|Default|SetIsInteracting false))

(event OnComponentBeginOverlap(MotionTrackerRange)
  (params (OverlappedComponent :type Primitive%20Component%20Object%20Reference) (OtherActor :type Actor%20Object%20Reference) (OtherComp :type Primitive%20Component%20Object%20Reference) (OtherBodyIndex :type Integer) (bFromSweep :type Boolean) (SweepResult :type Hit%20Result%20Structure%20%28by%20ref%29))
  ;[0.15 0.15 0.15 0.5] Motion Tracker
  (bind _asbp_enemy (Utilities|Casting|CastToBP_Enemy OtherActor))
  (Variables|Default|SetBP_Enemy _asbp_enemy))

(event OnComponentEndOverlap(MotionTrackerRange)
  (params (OverlappedComponent :type Primitive%20Component%20Object%20Reference) (OtherActor :type Actor%20Object%20Reference) (OtherComp :type Primitive%20Component%20Object%20Reference) (OtherBodyIndex :type Integer))
  ;[0.15 0.15 0.15 0.5] Motion Tracker
  (Variables|Default|SetBP_Enemy 0)
  (Audio|Parameter|SetFloatParameter (Variables|Default|GetMotionTrackerAudio) "Distance" 0.0 :!class /Script/Engine.AudioComponent))

(event Custom|ChangeColor_Event
  ;[0.15 0.15 0.15 0.5] Dynamic Material
  (Variables|Default|SetTargetProgress (Math|Float|SafeDivide (Math|Conversions|ToFloat(Integer) (Variables|/Game/Exercises/Blueprints/GM_EX.GM_EX_C|GetPoints (stale EventBeginPlay _asgm_ex))) (Math|Conversions|ToFloat(Integer) (Variables|/Game/Exercises/Blueprints/GM_EX.GM_EX_C|GetMaxPoints (stale EventBeginPlay _asgm_ex))))))

(event Input|EnhancedActionEvents|EnhancedInputActionIA_Interact
  (params (ActionValue :type Boolean) (ElapsedSeconds :type Float%20%28double-precision%29) (TriggeredSeconds :type Float%20%28double-precision%29) (InputAction :type Input%20Action%20Object%20Reference :default "/Game/Input/Actions/IA_Interact.IA_Interact"))
  ;[0.15 0.15 0.15 0.5] Interact
  (:Started
    (if (Variables|Default|GetIsInteracting)
      (bind _bp_interactable_base (Variables|Default|GetBP_Interactable%20Base)
        (:then
          (Default|Interact _bp_interactable_base))
        (:else)))))

(event Input|EnhancedActionEvents|EnhancedInputActionIA_Aim
  (params (ActionValue :type Boolean) (ElapsedSeconds :type Float%20%28double-precision%29) (TriggeredSeconds :type Float%20%28double-precision%29) (InputAction :type Input%20Action%20Object%20Reference :default "/Game/Input/Actions/IA_Aim.IA_Aim"))
  (bind _cameraboom (Variables|Default|GetCameraBoom))
  ;[0.15 0.15 0.15 0.5] Aim
  (:Triggered
    (Variables|/Script/Engine.SpringArmComponent|SetSocketOffset _cameraboom "0.000000,100.000000,0.000000")
    (Variables|/Script/Engine.SpringArmComponent|SetTargetArmLength _cameraboom 2e+02))
  (:Completed
    (Variables|/Script/Engine.SpringArmComponent|SetSocketOffset _cameraboom "0, 0, 0")
    (Variables|/Script/Engine.SpringArmComponent|SetTargetArmLength _cameraboom 4e+02)))

(event Input|EnhancedActionEvents|EnhancedInputActionIA_AIPickup
  (params (ActionValue :type Boolean) (ElapsedSeconds :type Float%20%28double-precision%29) (TriggeredSeconds :type Float%20%28double-precision%29) (InputAction :type Input%20Action%20Object%20Reference :default "/Game/Input/Actions/IA_AIPickup.IA_AIPickup"))
  (bind _followcamera (Variables|Default|GetFollowCamera))
  (bind _returnvalue (Transformation|GetWorldLocation _followcamera))
  ;[0.15 0.15 0.15 0.5] Event Pickup Request
  (:Started
    (bind (_outhit _returnvalue_2) (Collision|LineTraceByChannel _returnvalue (+ _returnvalue (* (Math|Vector|GetForwardVector _followcamera) (Variables|Default|GetDistance))) "TraceTypeQuery1" false 0 "None"))
    (if _returnvalue_2
      (bind _asbp_collectible_base (Utilities|Casting|CastToBP_CollectibleBase (.HitActor (Collision|BreakHitResult _outhit))))
      (Default|CallOnPickupRequest _asbp_collectible_base))))

(event EventBeginPlay
  ;[0.15 0.15 0.15 0.5] Dynamic Material
  (bind _asgm_ex (Utilities|Casting|CastToGM_EX (Game|GetGameMode)))
  (EventDispatchers|AssignUpdateGameBar _asgm_ex (delegate Custom|ChangeColor_Event)))

(event EventTick
  (params (DeltaSeconds :type Float%20%28single-precision%29))
  (Utilities|FlowControl|Sequence
    (:then_0
      ;[0.15 0.15 0.15 0.5] Motion Tracker
      (bind _bp_enemy (Variables|Default|GetBP_Enemy)
        (:then
          (Audio|Parameter|SetFloatParameter (Variables|Default|GetMotionTrackerAudio) "Distance" (|(1-(x/y)) (Transformation|GetDistanceTo _bp_enemy) 6e+02) :!class /Script/Engine.AudioComponent))
        (:else)))
    (:then_1
      ;[0.15 0.15 0.15 0.5] Smooth incremental game bar
      (bind _output_get (Variables|Default|SetCurrentProgress (Math|Interpolation|FInterpTo (Variables|Default|GetCurrentProgress) (Variables|Default|GetTargetProgress) DeltaSeconds 1.0)))
      (Rendering|Material|SetScalarParameterValue (Variables|Default|GetGameStateDynamicMaterial) "Progress" _output_get :!class /Script/Engine.MaterialInstanceDynamic))))

(fn ConstructionScript
  (|CallParentFunction)
  (bind _returnvalue (Rendering|Material|CreateDynamicMaterialInstance (Variables|Default|GetGameStateBar) 0 "/Game/Exercises/Materials/M_GameState.M_GameState" "None" :!class /Script/Engine.PrimitiveComponent))
  (Variables|Default|SetGameStateDynamicMaterial _returnvalue))