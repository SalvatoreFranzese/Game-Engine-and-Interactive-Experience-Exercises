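; GM_EX is an exercise game mode that tracks a points score and the win condition.
; On BeginPlay it creates the WBP_Overlay widget and adds it to the viewport.
; AddPoint increments Points, broadcasts PointsChanged with the value clamped to MaxPoints, and fires UpdateGameBar.
; When the clamped score reaches MaxPoints, it also shows the WBP_Won widget.
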(event `self.ReceiveBeginPlay`
  (bind _returnvalue (`|CreateWidget` "/Game/Exercises/Blueprints/UI/WBP_Overlay.WBP_Overlay_C"))
  (`UserWidget.AddToViewport` _returnvalue 0))

(fn `AddPoint`
  (bind _result (`/Engine/EditorBlueprintResources/StandardMacros.IncrementInt` (`self.Points`))
    (:`  `
      (bind _returnvalue (`KismetMathLibrary.Clamp` _result 0 (`self.MaxPoints`)))
      (`self.PointsChanged` _returnvalue)
      (if (< _returnvalue (`self.MaxPoints`))
        (`self.UpdateGameBar`)
        (else
          (`self.UpdateGameBar`)
          (bind _returnvalue_2 (`|CreateWidget` "/Game/Exercises/Blueprints/UI/WBP_Won.WBP_Won_C"))
          (`UserWidget.AddToViewport` _returnvalue_2 0))))))

(fn `UserConstructionScript`)